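; BP_GameDealer is a rhythm-game actor that spawns and manages moving beats and handles touch hits.
; Each beat spawns offset along X by 40% of viewport width, with move and scale speeds derived from the game instance's PLAYERDELAY.
; GameTick manually updates all beats, while touching the cylinder runs CheckBeat on each.
; Beat callbacks destroy scored or expired beats and relay scores through the AddScore dispatcher.
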(event `self.ReceiveBeginPlay`
  (`KismetSystemLibrary.Delay` 0.2)
  (`self.InitializeMe`))

(event `InitializeMe`
  (bind _returnvalue_x (`KismetMathLibrary.BreakVector2D` (`WidgetLayoutLibrary.GetViewportSize`)))
  (bind _returnvalue (* _returnvalue_x 0.4))
  (set `self.DealerDistance` _returnvalue)
  (`KismetSystemLibrary.PrintString` (`KismetStringLibrary.Concat_StrStr` "View Port Width x 0.4 : " (`KismetStringLibrary.Conv_DoubleToString` _returnvalue))))

(event `GameTick`
  (params (DeltalSec :type "Float (double-precision)"))
  (for _array_element (`self.AllSphereBeats`)
    (`/Game/Core/BP_GameDealerBeat.GameTick` _array_element DeltalSec)))

(event `SpawnNewBeat`
  (bind _returnvalue (`self.GetTransform`))
  (bind _asbp_main_game_inst (cast `/Game/Core/BP_MainGameInst` (`GameplayStatics.GetGameInstance`)))
  (bind _player_delay (`/Game/Core/BP_MainGameInst.PLAYER_DELAY` _asbp_main_game_inst))
  (bind _returnvalue_2 (`|SpawnActorFromClass` "/Game/Core/BP_GameDealerBeat.BP_GameDealerBeat_C" (`KismetMathLibrary.MakeTransform` (`KismetMathLibrary.MakeVector` (- (.x (.location _returnvalue)) (`self.DealerDistance`)) (.y (.location _returnvalue)) (.z (.location _returnvalue))) (.rotation _returnvalue) (.scale _returnvalue)) "Undefined" "OverrideRootScale" self (/ (`self.DealerDistance`) _player_delay) (/ 0.6 _player_delay) null))
  (add `/Game/Core/BP_GameDealerBeat.AddScore` _returnvalue_2 (delegate `AddScore_Event`))
  (add `/Game/Core/BP_GameDealerBeat.RemoveMe` _returnvalue_2 (delegate `RemoveMe_Event`))
  (`KismetArrayLibrary.Array_Add` (`self.AllSphereBeats`) _returnvalue_2))

(event `AddScore_Event`
  (params (Val :type "Float (double-precision)") (Beat :type "/Game/Core/BP_GameDealerBeat Object Reference"))
  (bind _allspherebeats (`self.AllSphereBeats`))
  (if (and (`KismetArrayLibrary.Array_Contains` _allspherebeats Beat) (> Val 0.0))
    (`self.K2_DestroyActor` Beat)
    (`KismetArrayLibrary.Array_RemoveItem` _allspherebeats Beat))
  (`self.AddScore` Val))

(event `RemoveMe_Event`
  (params (Beat :type "/Game/Core/BP_GameDealerBeat Object Reference"))
  (bind _allspherebeats (`self.AllSphereBeats`))
  (if (`KismetArrayLibrary.Array_Contains` _allspherebeats Beat)
    (`self.K2_DestroyActor` Beat)
    (`KismetArrayLibrary.Array_RemoveItem` _allspherebeats Beat)))

(event `self.Cylinder.OnInputTouchBegin`
  (params (FingerIndex :type "ETouchIndex Enum" :default "Touch1") (TouchedComponent :type "PrimitiveComponent Object Reference"))
  (for _array_element (`self.AllSphereBeats`)
    (`/Game/Core/BP_GameDealerBeat.CheckBeat` _array_element)))

(fn `UserConstructionScript`)