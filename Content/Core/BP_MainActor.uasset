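; Main actor of a rhythm game that runs a session from song pick through scoring, pause and game over.
; The picked song's OnsetNRT asset loads synchronously, and its channel 0 onsets become a beat list rounded down to tenths of a second.
; Audio playback percent is matched against that list to make the child-actor BP_GameDealer spawn beats and report score changes.
; When the audio finishes, it shows the game-over widget and saves a history record.
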(event `self.ReceiveBeginPlay`
  (bind _asbp_game_dealer (cast `/Game/Core/BP_GameDealer` (`ChildActorComponent.ChildActor` (`self.BP_GameDealer`))))
  (bind _output_get (set `self.MainDealer` _asbp_game_dealer))
  (add `/Game/Core/BP_GameDealer.AddScore` _output_get (delegate `AddScore_Event`))
  (bind _returnvalue (`|CreateWidget` "/Game/UI/PickOneSong/WBP_PickSongUI.WBP_PickSongUI_C"))
  (add `/Game/UI/PickOneSong/WBP_PickSongUI.SongSoftPathArrived` _returnvalue (delegate `SongSoftPathArrived_Event`))
  (`/Game/UI/PickOneSong/WBP_PickSongUI.ShowMe` _returnvalue self))

(event `AddScore_Event`
  (params (Val :type "Float (double-precision)"))
  (if (`KismetSystemLibrary.IsValid` (`self.MainUMG`))
    (bind _output_get (set `self.CurrScore` (`KismetMathLibrary.FClamp` (+ Val (`self.CurrScore`)) 0.0 999999.0)))
    (`/Game/UI/WBP_MainUMG.UpdScore` (`self.MainUMG`) _output_get)))

(event `SongSoftPathArrived_Event`
  (params (OnsetSoftPath :type String))
  (bind _output_get (set `self.CurrOnsetSoftPath` OnsetSoftPath))
  (`KismetSystemLibrary.DelayUntilNextTick`)
  (set `self.CurrOnsetNRT` (`self.LoadOneOnsetParser` _output_get))
  (`self.StartPlayGame`))

(event `self.ReceiveTick`
  (params (DeltaSeconds :type "Float (single-precision)"))
  (if (not (`self.IsPauseGame`))
    (`/Game/Core/BP_GameDealer.GameTick` (`self.MainDealer`) DeltaSeconds)))

(event `TogglePauseSong_Event`
  (params (IsPause :type Boolean))
  (bind _currsound2d (`self.CurrSound2D`))
  (bind _output_get (set `self.IsPauseGame` IsPause))
  (if (`KismetSystemLibrary.IsValid` _currsound2d)
    (`AudioComponent.SetPaused` _currsound2d _output_get)))

(event `StartPlayGame`
  (bind _returnvalue (`|CreateWidget` "/Game/UI/WBP_MainUMG.WBP_MainUMG_C"))
  (bind _output_get (set `self.MainUMG` _returnvalue))
  (add `/Game/UI/WBP_MainUMG.StartPlayGame` _output_get (delegate `StartPlayGame_Event`))
  (add `/Game/UI/WBP_MainUMG.TogglePauseSong` _output_get (delegate `TogglePauseSong_Event`))
  (`/Game/UI/WBP_MainUMG.ShowMe` _output_get))

(event `StartPlayGame_Event`
  (bind _sound (`AudioAnalyzerNRT.Sound` (`self.CurrOnsetNRT`)))
  (set `self.CurrSongDuration` (`SoundBase.Duration` _sound))
  (bind _returnvalue (`GameplayStatics.SpawnSound2D` _sound 1.0 1.0 0.0 null))
  (bind _output_get (set `self.CurrSound2D` _returnvalue))
  (`AudioComponent.Stop` _output_get)
  (add `AudioComponent.OnAudioFinished` _output_get (delegate `OnAudioFinished_Event`))
  (add `AudioComponent.OnAudioPlaybackPercent` _output_get (delegate `OnAudioPlaybackPercent_Event`))
  (`AudioComponent.Play` _output_get 0.0)
  (`/Game/UI/WBP_MainUMG.EnablePauseBtn` (`self.MainUMG`))
  (`self.FindBeats5SecondsStep2` 0.0 (`self.CurrSongDuration`) (`self.BeatsInTimestamp`))
  (bind _asbp_game_dealer (cast `/Game/Core/BP_GameDealer` (`ChildActorComponent.ChildActor` (`self.BP_GameDealer`))))
  (`/Game/Core/BP_GameDealer.InitializeMe` _asbp_game_dealer))

(event `OnAudioFinished_Event`
  (`self.SongFinishedEvt`))

(event `OnAudioPlaybackPercent_Event`
  (params (PlayingSoundWave :type "SoundWave Object Reference") (PlaybackPercent :type "Float (single-precision)"))
  (bind _beatsintimestamp (`self.BeatsInTimestamp`))
  (bind _returnvalue (`self.OneDigitalFraction` (* (`self.CurrSongDuration`) PlaybackPercent)))
  (if (`KismetArrayLibrary.Array_Contains` _beatsintimestamp _returnvalue)
    (`KismetArrayLibrary.Array_RemoveItem` _beatsintimestamp _returnvalue)
    (`/Game/Core/BP_GameDealer.SpawnNewBeat` (`self.MainDealer`))))

(event `SongFinishedEvt`
  ; Gameover and show Statistics Window
  (bind _returnvalue (`|CreateWidget` "/Game/UI/WBP_Gameover.WBP_Gameover_C"))
  (`/Game/UI/WBP_Gameover.ShowMe` _returnvalue)
  (`self.UpdSaveData`)
  (message `/Game/Core/BPI_GameInst.SaveGameNow` (cast `/Game/Core/BP_MainGameInst` (`GameplayStatics.GetGameInstance`) :!pure true)))

(fn `FindBeats5SecondsStep`
  (params (CurrTime :type "Float (double-precision)") (MaxTime :type "Float (double-precision)") (OutputArray :type "Array of Float (double-precision)"))
  (locals (IsLoop :type Boolean :default true) (TmpTime :type "Float (double-precision)"))
  (bind _output_get (set `local.TmpTime` CurrTime))
  (while (and (`local.IsLoop`) (< (`KismetArrayLibrary.Array_Length` OutputArray) 10))
    (bind _returnvalue (`KismetMathLibrary.FClamp` (+ _output_get 5.0) 0.0 MaxTime))
    (for _array_element (`OnsetNRT.GetNormalizedChannelOnsetsBetweenTimes` (`self.CurrOnsetNRT`) _output_get _returnvalue 0)
      (`KismetArrayLibrary.Array_AddUnique` OutputArray (`self.OneDigitalFraction` _array_element)))
    (if (>= _returnvalue MaxTime)
      (set `local.IsLoop` false)
      (set `local.TmpTime` _returnvalue))))

(fn `FindBeats5SecondsStep2`
  (params (CurrTime :type "Float (double-precision)") (MaxTime :type "Float (double-precision)") (OutputArray :type "Array of Float (double-precision)"))
  (locals (IsLoop :type Boolean :default true) (TmpTime :type "Float (double-precision)"))
  (for _array_element (`OnsetNRT.GetNormalizedChannelOnsetsBetweenTimes` (`self.CurrOnsetNRT`) 0.0 MaxTime 0)
    (`KismetArrayLibrary.Array_AddUnique` OutputArray (`self.OneDigitalFraction` _array_element))))

(fn `LoadOneOnsetParser`
  (params (SoftPath :type String))
  (returns (RslOnsetNRT :type "OnsetNRT Object Reference"))
  (bind _returnvalue (`KismetSystemLibrary.LoadAsset_Blocking` (`KismetSystemLibrary.Conv_SoftObjPathToSoftObjRef` (`KismetSystemLibrary.MakeSoftObjectPath` SoftPath))))
  (bind _asonset_nrt (cast `OnsetNRT` _returnvalue))
  (return _asonset_nrt))

(fn `OneDigitalFraction`
  (params (A :type "Float (double-precision)"))
  (returns (ReturnValue :type "Float (double-precision)"))
  (return (* (`KismetMathLibrary.FFloor` (* A 10.0)) 0.1)))

(fn `UpdSaveData`
  (bind _gameinst (`/Game/Core/BPF_CommFuncs.GameInst`))
  (`KismetArrayLibrary.Array_Add` (`/Game/Core/SaveGame/BP_SaveGame.HistoryRecords` (`/Game/Core/BP_MainGameInst.TOOTSaveDat` _gameinst)) (make `/Game/Core/SaveGame/ST_SaveData` (`/Game/Core/BP_MainGameInst.CurrPlayerName` _gameinst) (`KismetTextLibrary.Conv_StringToText` (`/Game/Core/BP_MainGameInst.CurrSongName` _gameinst)) (`KismetMathLibrary.FTrunc` (`self.CurrScore`)) (`KismetMathLibrary.ToUnixTimestamp` (`KismetMathLibrary.UtcNow`)))))

(fn `UserConstructionScript`)