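; Game instance Blueprint that catalogs the project's Audio Synesthesia OnsetNRT assets at startup.
; After a short delay, Init queries the Asset Registry by class, including subclasses, and stores each asset's object path string in AllOnSetObjPaths.
; The FC event prints the stored paths for debugging.
; An unconnected fragment sketches a name-matched blocking load that prints the onset asset's sound duration.
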(event `self.ReceiveInit`
  (`KismetSystemLibrary.Delay` 0.1)
  (bind _outassetdata (`AssetRegistry.GetAssetsByClass` (`AssetRegistryHelpers.GetAssetRegistry`) (`KismetSystemLibrary.MakeTopLevelAssetPath` (`KismetSystemLibrary.BreakTopLevelAssetPath` (`KismetSystemLibrary.GetClassTopLevelAssetPath` "/Script/AudioSynesthesia.OnsetNRT"))) true))
  (for _array_element _outassetdata
    (bind (_packagename _packagepath _assetname) (break `AssetData` _array_element))
    (`KismetArrayLibrary.Array_Add` (`self.AllOnSetObjPaths`) (`KismetStringLibrary.Concat_StrStr` (`KismetStringLibrary.Conv_NameToString` _packagename) "." (`KismetStringLibrary.Conv_NameToString` _assetname)))))

(event `FC`
  (for _array_element (`self.AllOnSetObjPaths`)
    (`KismetSystemLibrary.PrintString` _array_element)))