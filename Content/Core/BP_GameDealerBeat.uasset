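; Rhythm-game beat actor whose sphere slides along X and can be scored inside a timing window around X = 0.
; A custom GameTick event moves the sphere, growing it before zero and shrinking it after.
; CheckBeat reports +1 within the GameInstance's distance threshold.
; Passing the threshold applies the failed material and reports -1 once, then requests removal when scale drops below zero.
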(event `self.ReceiveBeginPlay`
  (bind _asbp_main_game_inst (cast `/Game/Core/BP_MainGameInst` (`GameplayStatics.GetGameInstance`)))
  (set `self.DistanceThreshold` (`/Game/Core/BP_MainGameInst.BEAT_DISTANCE_THRESHOLD` _asbp_main_game_inst)))

(event `GameTick`
  (params (DeltalSec :type "Float (double-precision)"))
  (bind _returnvalue_x (`KismetMathLibrary.BreakVector` (`self.K2_GetActorLocation`)))
  (bind _returnvalue_x_2 (`KismetMathLibrary.BreakVector` (`self.K2_GetActorLocation`)))
  (bind _curr3dsize (`self.Curr3DSize`))
  (bind _curr3dsize_2 (`self.Curr3DSize`))
  (bind _returnvalue (* (`self.ScaleSpeed`) DeltalSec))
  (`SceneComponent.K2_AddRelativeLocation` (`self.Sphere`) (`KismetMathLibrary.MakeVector` (* DeltalSec (`self.MoveSpeed`))) false false)
  (if (< _returnvalue_x_2 0.0)
    (set `self.Curr3DSize` (+ _returnvalue _curr3dsize_2))
    (else
      (set `self.Curr3DSize` (- _curr3dsize_2 _returnvalue))))
  (`SceneComponent.SetRelativeScale3D` (`self.Sphere`) (`KismetMathLibrary.MakeVector` _curr3dsize _curr3dsize _curr3dsize))
  (if (> _returnvalue_x (`self.DistanceThreshold`))
    (if (< (`self.Curr3DSize`) 0.0)
      (`self.RemoveMe` self)
      (else
        (`/Engine/EditorBlueprintResources/StandardMacros.DoOnce` false
          (:`Completed`
            (`PrimitiveComponent.SetMaterial` (`self.Sphere`) 0 "/Game/Materials/M_DealerBeat_Failed.M_DealerBeat_Failed")
            (`self.AddScore` -1.0 self)))))))

(fn `CheckBeat`
  (if (`self.IsInside`)
    (`self.AddScore` 1.0 self)))

(fn `IsInside`
  (returns (IsIn :type Boolean))
  (bind _returnvalue_x (`KismetMathLibrary.BreakVector` (`self.K2_GetActorLocation`)))
  (bind _distancethreshold (`self.DistanceThreshold`))
  (if (or (< _returnvalue_x (* _distancethreshold -1.0)) (> _returnvalue_x _distancethreshold))
    (return false)
    (else
      (return true))))

(fn `UserConstructionScript`)